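; Circular spline actor that procedurally lays out a ring of spline points from Segments and Radius, with Radius scaled by 100.
; The construction script clears CircleSpline, then spaces points evenly around the local origin using sine and cosine.
; Each tangent is perpendicular to the center direction, scaled by a tangent-based arc approximation that uses 350 degrees rather than 360.
; Event graph logic is empty.
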(event EventBeginPlay)

(event Collision|EventActorBeginOverlap
  (params (OtherActor :type Actor%20Object%20Reference)))

(event EventTick
  (params (DeltaSeconds :type Float%20%28single-precision%29)))

(fn ConstructionScript
  (bind _circle_spline (Variables|Default|GetCircle%20Spline))
  (bind _radius (Variables|Default|GetRadius))
  (bind _segments (Variables|Default|GetSegments))
  (bind _returnvalue (- _segments 1))
  (bind _returnvalue_2 (* _radius 1e+02))
  (Spline|ClearSplinePoints (Variables|Default|GetCircle%20Spline) true)
  (if (> _segments 0)
    (for _index (range 0 _returnvalue)
      (Spline|AddSplinePoint _circle_spline (Math|Vector|MakeVector (* (Math|Trig|Sin(Degrees) (Math|Float|MapRangeClamped (Math|Conversions|ToFloat(Integer) _index) 0.0 (Math|Conversions|ToFloat(Integer) _returnvalue) 0.0 (Math|Conversions|ToFloat(Integer) (|(360-(360/vSegments)) _segments)))) _returnvalue_2) (* (Math|Trig|Cos(Degrees) (Math|Float|MapRangeClamped (Math|Conversions|ToFloat(Integer) _index) 0.0 (Math|Conversions|ToFloat(Integer) _returnvalue) 0.0 (Math|Conversions|ToFloat(Integer) (|(360-(360/vSegments)) _segments)))) _returnvalue_2) 0.0) "Local" true)
      (Spline|SetTangentatSplinePoint _circle_spline _index (* (Math|Vector|GetRightVector (Math|Rotator|FindLookatRotation (Math|Vector|MakeVector (* (Math|Trig|Sin(Degrees) (Math|Float|MapRangeClamped (Math|Conversions|ToFloat(Integer) _index) 0.0 (Math|Conversions|ToFloat(Integer) _returnvalue) 0.0 (Math|Conversions|ToFloat(Integer) (|(360-(360/vSegments)) _segments)))) _returnvalue_2) (* (Math|Trig|Cos(Degrees) (Math|Float|MapRangeClamped (Math|Conversions|ToFloat(Integer) _index) 0.0 (Math|Conversions|ToFloat(Integer) _returnvalue) 0.0 (Math|Conversions|ToFloat(Integer) (|(360-(360/vSegments)) _segments)))) _returnvalue_2) 0.0) (Math|Vector|MakeVector 0.0 0.0 0.0))) (* _returnvalue_2 (|(4*(tan(((D2R((350/vSegments)))/4)))) _segments))) "Local" true)))
  (Spline|UpdateSpline (Variables|Default|GetCircle%20Spline)))